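; AI pawn Blueprint that plays a male pain grunt chosen by the body part that was hit.
; BeginPlay assigns the head, body and leg sounds.
; The GotHit event maps the bone name to one of them (clavicles and spine as body, thighs as leg), then plays it as non-spatial 2D audio.
; Unmatched bones leave the previous HitSound in place, which still plays.
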(event EventBeginPlay
  (Variables|Default|SetHeadHitSound "/Game/HumanVocalizations/HumanMaleA/Wavs/voice_male_grunt_pain_05.voice_male_grunt_pain_05")
  (Variables|Default|SetBodyHitSound "/Game/HumanVocalizations/HumanMaleA/Wavs/voice_male_grunt_pain_03.voice_male_grunt_pain_03")
  (Variables|Default|SetLegHitSound "/Game/HumanVocalizations/HumanMaleA/Wavs/voice_male_grunt_pain_01.voice_male_grunt_pain_01"))

(event Collision|EventActorBeginOverlap
  (params (OtherActor :type Actor%20Object%20Reference)))

(event EventTick
  (params (DeltaSeconds :type Float%20%28single-precision%29)))

(event EventGotHit
  (params (BoneName :type Name :default "None"))
  (Utilities|FlowControl|Sequence
    (:then_0
      (switch string (Utilities|String|ToString(Name) BoneName)
        (:head
          (Variables|Default|SetHitSound (Variables|Default|GetHeadHitSound)))
        (:clavicle_l
          (Variables|Default|SetHitSound (Variables|Default|GetBodyHitSound) :!label _label))
        (:clavicle_r
          (goto _label))
        (:spine_01
          (goto _label))
        (:spine_02
          (goto _label))
        (:spine_03
          (goto _label))
        (:thigh_l
          (Variables|Default|SetHitSound (Variables|Default|GetLegHitSound) :!label _label_2))
        (:thigh_r
          (goto _label_2))))
    (:then_1
      (Audio|PlaySound2D (Variables|Default|GetHitSound) 1.0 1.0 0.0 0 0))))

(fn ConstructionScript)