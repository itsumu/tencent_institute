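; BP_AICharacter is an AI character that carries a rifle, can fire it and reacts to being hit.
; BeginPlay spawns a BP_Rifle_Master, attaches it to the mesh's GripPoint socket and registers itself as shooter.
; Fire aims the muzzle along the weapon mesh's right vector before starting fire.
; GotHit sets a Hurt flag and plays a non-spatial pain sound chosen by bone name, and a helper sets walk speed.
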(event EventBeginPlay
  ;[1 1 1] Begin play
  (Variables|Default|SetHeadHitSound "/Game/HumanVocalizations/HumanMaleA/Wavs/voice_male_grunt_pain_05.voice_male_grunt_pain_05")
  (Variables|Default|SetBodyHitSound "/Game/HumanVocalizations/HumanMaleA/Wavs/voice_male_grunt_pain_03.voice_male_grunt_pain_03")
  (Variables|Default|SetLegHitSound "/Game/HumanVocalizations/HumanMaleA/Wavs/voice_male_grunt_pain_01.voice_male_grunt_pain_01")
  ;[1 1 1] Arm weapon
  (bind _returnvalue (Game|SpawnActorfromClass "/Game/Blueprints/Weapons/BP_Rifle_Master.BP_Rifle_Master_C" (Math|Transform|MakeTransform "0, 0, 0") "AlwaysSpawn" 0 0))
  (bind _output_get (Variables|Default|SetEquippedGun _returnvalue))
  (Transformation|AttachComponentToComponent _output_get (Variables|Character|GetMesh) "GripPoint" "SnapToTarget" "SnapToTarget" "SnapToTarget" true)
  (Variables|/Script/TencentSchool.Gun|SetShooter _output_get self))

(event Collision|EventActorBeginOverlap
  (params (OtherActor :type Actor%20Object%20Reference)))

(event EventTick
  (params (DeltaSeconds :type Float%20%28single-precision%29)))

(event EventGotHit
  (params (BoneName :type Name :default "None"))
  (CallFunction|Groan BoneName)
  (Variables|Default|SetHurt true))

(fn ConstructionScript)

(fn UpdateMovementSpeed
  (params (NewWalkSpeed :type Float%20%28single-precision%29))
  (Variables|/Script/Engine.CharacterMovementComponent|SetMaxWalkSpeed (Variables|Character|GetCharacterMovement) NewWalkSpeed))

(fn SetMuzzleRotation
  (bind _equippedgun (Variables|Default|GetEquippedGun))
  (bind _returnvalue (Actor|GetComponentbyClass _equippedgun "/Script/Engine.SkeletalMeshComponent"))
  (bind _returnvalue_2 (Transformation|GetSocketLocation _returnvalue "Muzzle"))
  (Variables|/Script/TencentSchool.Gun|SetMuzzleRotation _equippedgun (Math|Rotator|FindLookatRotation _returnvalue_2 (+ _returnvalue_2 (Math|Vector|GetRightVector _returnvalue)))))

(fn Fire
  (CallFunction|SetMuzzleRotation)
  (Class|Gun|StartFire (Variables|Default|GetEquippedGun) self))

(fn Groan
  (params (BoneName :type Name))
  (Utilities|FlowControl|Sequence
    (:then_0
      (switch string (Utilities|String|ToString(Name) BoneName)
        (:Default
          (Variables|Default|SetHitSound "/Game/HumanVocalizations/HumanMaleD/Cues/voice_male_d_hurt_pain_05_Cue.voice_male_d_hurt_pain_05_Cue"))
        (:head
          (Variables|Default|SetHitSound (Variables|Default|GetHeadHitSound)))
        (:clavicle_l
          (Variables|Default|SetHitSound (Variables|Default|GetBodyHitSound) :!label _label))
        (:clavicle_r
          (goto _label))
        (:spine_01
          (goto _label))
        (:spine_02
          (goto _label))
        (:spine_03
          (goto _label))
        (:thigh_l
          (Variables|Default|SetHitSound (Variables|Default|GetLegHitSound) :!label _label_2))
        (:thigh_r
          (goto _label_2))))
    (:then_1
      (Audio|PlaySound2D (Variables|Default|GetHitSound) 1.0 1.0 0.0 0 0))))